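; Game mode Blueprint that handles respawning a given controller's character.
; Its Respawn event destroys any currently controlled pawn, then spawns a new ThirdPersonCharacter at a randomly chosen PlayerStart and has the controller possess it.
; The spawn adjusts for collisions but always succeeds, and nothing in this Blueprint calls Respawn, as BeginPlay and Tick are unused.
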(event `/Game/BPI_GameMode.Respawn`
  (params (Controller :type "Controller Object Reference"))
  (bind _returnvalue (`Controller.K2_GetPawn` Controller))
  (`/Engine/EditorBlueprintResources/StandardMacros.IsValid` _returnvalue
    (:`Is Valid`
      (`self.K2_DestroyActor` _returnvalue))
    (:`Is Not Valid`
      _))
  (bind _outactors (`GameplayStatics.GetAllActorsOfClass` "/Script/Engine.PlayerStart"))
  (bind _returnvalue_2 (`|SpawnActorFromClass` "/Game/ThirdPersonCPP/Blueprints/ThirdPersonCharacter.ThirdPersonCharacter_C" (`self.GetTransform` (`|GetArrayItem` _outactors (`KismetMathLibrary.RandomIntegerInRange` 0 (- (`KismetArrayLibrary.Array_Length` _outactors) 1)))) "AdjustIfPossibleButAlwaysSpawn" "OverrideRootScale" null null))
  (`Controller.Possess` Controller _returnvalue_2))

(fn `UserConstructionScript`)