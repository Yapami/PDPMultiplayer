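; Player controller that applies the saved character sex to the possessed pawn and handles menu and scoreboard input.
; On authority possession, LocalChangeSex reads the PlayerInfo save and passes Sex to ServerChangeSex, which sets it on the ThirdPersonCharacter; SetMesh also calls ServerChangeSex.
; MainMenu input flip-flops the MyHUD menu, mouse cursor and pawn input.
; ScoreBoard input shows the HUD scoreboard while held.
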(event `LocalChangeSex`
  (bind _returnvalue (`GameplayStatics.LoadGameFromSlot` "PlayerInfo"))
  (bind _aspdp_player_saved_info (cast `/Game/Start/PDP_PlayerSavedInfo` _returnvalue))
  (`self.ServerChangeSex` (`/Game/Start/PDP_PlayerSavedInfo.Sex` _aspdp_player_saved_info)))

(event `ServerChangeSex`
  (params (Sex :type Boolean))
  (bind _asthird_person_character (cast `/Game/ThirdPersonCPP/Blueprints/ThirdPersonCharacter` (`self.K2_GetPawn`)))
  (set `/Game/ThirdPersonCPP/Blueprints/ThirdPersonCharacter.Sex` Sex _asthird_person_character))

(event `self.ReceivePossess`
  (params (PossessedPawn :type "Pawn Object Reference"))
  (`/Engine/EditorBlueprintResources/ActorMacros.Switch Has Authority`
    (:`Authority`
      (`self.LocalChangeSex`))))

(event `self.ReceiveBeginPlay`
  (`WidgetBlueprintLibrary.SetInputMode_GameOnly` self))

(event `InputAction|MainMenu`
  (params (Key :type "Key Structure"))
  (bind _returnvalue (`self.K2_GetPawn`))
  (:`Pressed`
    (`/Engine/EditorBlueprintResources/StandardMacros.FlipFlop`
      (:`A`
        (bind _asmy_hud (cast `/Game/UI/MyHUD` (`self.GetHUD`)))
        (`/Game/UI/MyHUD.Draw Main Menu` _asmy_hud)
        (set `self.bShowMouseCursor` true)
        (`self.DisableInput` _returnvalue self))
      (:`B`
        (bind _asmy_hud_2 (cast `/Game/UI/MyHUD` (`self.GetHUD`)))
        (`/Game/UI/MyHUD.Delete Main Menu` _asmy_hud_2)
        (set `self.bShowMouseCursor` false)
        (`self.EnableInput` _returnvalue self)))))

(event `InputAction|ScoreBoard`
  (params (Key :type "Key Structure"))
  (:`Pressed`
    (bind _asmy_hud (cast `/Game/UI/MyHUD` (`self.GetHUD`)))
    (`/Game/UI/MyHUD.ShowScoreBoard` _asmy_hud))
  (:`Released`
    (bind _asmy_hud_2 (cast `/Game/UI/MyHUD` (`self.GetHUD`)))
    (`/Game/UI/MyHUD.CloseScoreBoard` _asmy_hud_2)))

(fn `SetMesh`
  (params (Sex :type Boolean))
  (`self.ServerChangeSex` Sex))

(fn `UserConstructionScript`)